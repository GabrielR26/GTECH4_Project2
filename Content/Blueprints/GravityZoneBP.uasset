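; Gravity zone actor that overrides gravity on the static mesh components of actors inside it.
; Overlap begin disables each mesh's built-in gravity and adds it to a tracked list; overlap end restores gravity and removes it.
; Each tick applies a mass-scaled force to tracked meshes, with GetGravityForce choosing upward, zero or downward gravity from the GravityType enum.
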(event `self.ReceiveTick`
  (params (DeltaSeconds :type "Float (single-precision)"))
  (for _array_element (`self.allActorInZone`)
    (`/Engine/EditorBlueprintResources/StandardMacros.IsValid` _array_element
      (:`Is Valid`
        (bind _force (`self.GetGravityForce`))
        (`PrimitiveComponent.AddForce` _array_element (* _force (`PrimitiveComponent.GetMass` _array_element)) "None" false)))))

(event `self.ReceiveActorBeginOverlap`
  (params (OtherActor :type "Actor Object Reference"))
  (bind _returnvalue (`self.GetComponentByClass` OtherActor "/Script/Engine.StaticMeshComponent"))
  (`/Engine/EditorBlueprintResources/StandardMacros.IsValid` OtherActor
    (:`Is Valid`
      (`/Engine/EditorBlueprintResources/StandardMacros.IsValid` _returnvalue
        (:`Is Valid`
          (`PrimitiveComponent.SetEnableGravity` _returnvalue false)
          (`KismetArrayLibrary.Array_Add` (`self.allActorInZone`) _returnvalue))))))

(event `self.ReceiveActorEndOverlap`
  (params (OtherActor :type "Actor Object Reference"))
  (bind _returnvalue (`self.GetComponentByClass` OtherActor "/Script/Engine.StaticMeshComponent"))
  (`/Engine/EditorBlueprintResources/StandardMacros.IsValid` OtherActor
    (:`Is Valid`
      (`/Engine/EditorBlueprintResources/StandardMacros.IsValid` _returnvalue
        (:`Is Valid`
          (`PrimitiveComponent.SetEnableGravity` _returnvalue true)
          (`KismetArrayLibrary.Array_RemoveItem` (`self.allActorInZone`) _returnvalue))))))

(fn `GetGravityForce`
  (returns (force :type "Vector Structure"))
  (bind _gravitytype (`self.gravityType`))
  (if (`|EnumEquality` _gravitytype "NewEnumerator0")
    (return (0.0 0.0 980.0))
    (elif (`|EnumEquality` _gravitytype "NewEnumerator1")
      (return (0.0 0.0 0.0))
      (else
        (return (0.0 0.0 -980.0))))))

(fn `UserConstructionScript`)